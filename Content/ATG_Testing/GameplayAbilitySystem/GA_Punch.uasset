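; GA_Punch is a Gameplay Ability that plays an attack montage and applies GE_Damage when a hit is reported.
; While the montage runs, a one-shot WaitGameplayEvent task listens for Reub.Weapon.Hit and applies the damage effect to the event payload's target data.
; Montage completion, blend-out or interruption ends the ability, and OnEndAbility ends the stored wait task if still valid.
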(event `self.K2_ActivateAbility`
  (bind (_returnvalue_owneractor _returnvalue_avataractor _returnvalue_playercontroller _returnvalue_abilitysystemcomponent _returnvalue_skeletalmeshcomponent) (break `GameplayAbilityActorInfo` (`self.GetActorInfo`)))
  (`|PlayMontage` _returnvalue_skeletalmeshcomponent "/Game/ATG_Testing/GameplayAbilitySystem/Animations/M_AttackReMake.M_AttackReMake"
    (:`then`
      (bind (_asynctaskproxy _payload) (`AbilityTask_WaitGameplayEvent.WaitGameplayEvent` (struct :`TagName` "Reub.Weapon.Hit") null true)
        (:`then`
          (set `self.Async Task Variable` _asynctaskproxy))
        (:`EventReceived`
          (`self.BP_ApplyGameplayEffectToTarget` (`.TargetData` (break `GameplayEventData` _payload)) "/Game/ATG_Testing/GameplayAbilitySystem/GE_Damage.GE_Damage_C"))))
    (:`OnCompleted`
      (`KismetSystemLibrary.PrintString` "Ability Triggered" :!label _label)
      (`self.K2_EndAbility`))
    (:`OnBlendOut`
      (goto _label))
    (:`OnInterrupted`
      (goto _label))))

(event `self.K2_OnEndAbility`
  (params (bWasCancelled :type Boolean))
  (bind _async_task_variable (`self.Async Task Variable`))
  (`/Engine/EditorBlueprintResources/StandardMacros.IsValid` _async_task_variable
    (:`Is Valid`
      (`GameplayTask.EndTask` _async_task_variable))))