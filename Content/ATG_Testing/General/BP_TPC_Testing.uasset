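; Test third-person character combining parkour movement, Gameplay Ability System melee and an inventory screen.
; BeginPlay adds the Enhanced Input mapping and applies GE_Damage to itself; movement inputs, landing and mode changes feed ParkourMovementSystem.
; Punch input activates GA_Punch, while HandlePunch sphere-overlaps at the right hand and sends a hit gameplay event with target data.
; Helmet and vest meshes follow the body via leader pose.
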(event `self.ReceiveBeginPlay`
  (bind _asplayer_controller (cast `PlayerController` (`self.GetController`)))
  (bind _returnvalue (pcsubsystem `EnhancedInputLocalPlayerSubsystem` _asplayer_controller))
  (`/Engine/EditorBlueprintResources/StandardMacros.IsValid` _returnvalue
    (:`Is Valid`
      (`EnhancedInputSubsystemInterface.AddMappingContext` _returnvalue "/Game/ATG_Testing/Collab/IM_Collab_Controls.IM_Collab_Controls" 0 (struct))
      (`AbilitySystemComponent.BP_ApplyGameplayEffectToSelf` :`self` (`self.AbilitySystemComponent`) :`GameplayEffectClass` "/Game/ATG_Testing/GameplayAbilitySystem/GE_Damage.GE_Damage_C" :`Level` 1.0))))

(event `self.ReceiveTick`
  (params (DeltaSeconds :type "Float (single-precision)")))

(event `self.K2_OnMovementModeChanged`
  (params (PrevMovementMode :type "EMovementMode Enum" :default "MOVE_None") (NewMovementMode :type "EMovementMode Enum" :default "MOVE_None") (PrevCustomMode :type Byte) (NewCustomMode :type Byte))
  (`ParkourMovementComponent.MovementChanged` (`self.ParkourMovementSystem`) PrevMovementMode NewMovementMode)
  (`KismetSystemLibrary.PrintString` (`|GetEnumeratorNameAsString` NewMovementMode)))

(event `EnhancedInput|/Game/ATG_Testing/TargetSystem/IA_Target`
  (params (ActionValue :type Boolean) (ElapsedSeconds :type "Float (double-precision)") (TriggeredSeconds :type "Float (double-precision)") (InputAction :type "InputAction Object Reference" :default "/Game/ATG_Testing/TargetSystem/IA_Target.IA_Target")))

(event `EnhancedInput|/Game/ATG_Testing/InventorySystem/IA_OpenInventory`
  (params (ActionValue :type Boolean) (ElapsedSeconds :type "Float (double-precision)") (TriggeredSeconds :type "Float (double-precision)") (InputAction :type "InputAction Object Reference" :default "/Game/ATG_Testing/InventorySystem/IA_OpenInventory.IA_OpenInventory"))
  (bind _returnvalue (`GameplayStatics.GetPlayerController` 0))
  (:`Triggered`
    (bind _returnvalue_2 (`|CreateWidget` "/Game/ATG_Testing/InventorySystem/WBP_Inventory.WBP_Inventory_C" _returnvalue))
    (`UserWidget.AddToViewport` _returnvalue_2 0)
    (set `PlayerController.bShowMouseCursor` true _returnvalue)
    (`WidgetBlueprintLibrary.SetInputMode_UIOnlyEx` _returnvalue _returnvalue_2)))

(event `EnhancedInput|/Game/ThirdPerson/Input/Actions/IA_Jump`
  (params (ActionValue :type Boolean) (ElapsedSeconds :type "Float (double-precision)") (TriggeredSeconds :type "Float (double-precision)") (InputAction :type "InputAction Object Reference" :default "/Game/ThirdPerson/Input/Actions/IA_Jump.IA_Jump"))
  (:`Triggered`
    (`self.Jump`)
    (`ParkourMovementComponent.Jump` (`self.ParkourMovementSystem`)))
  (:`Completed`
    (`self.StopJumping`)))

(event `EnhancedInput|/Game/ATG_Testing/ParkourMovement/IA_Crouch`
  (params (ActionValue :type Boolean) (ElapsedSeconds :type "Float (double-precision)") (TriggeredSeconds :type "Float (double-precision)") (InputAction :type "InputAction Object Reference" :default "/Game/ATG_Testing/ParkourMovement/IA_Crouch.IA_Crouch"))
  (:`Triggered`
    (`ParkourMovementComponent.CrouchSlide` (`self.ParkourMovementSystem`))))

(event `self.OnLanded`
  (params (Hit :type "HitResult Structure (by ref)"))
  (`ParkourMovementComponent.Land` (`self.ParkourMovementSystem`)))

(event `EnhancedInput|/Game/ATG_Testing/ParkourMovement/IA_Sprint`
  (params (ActionValue :type Boolean) (ElapsedSeconds :type "Float (double-precision)") (TriggeredSeconds :type "Float (double-precision)") (InputAction :type "InputAction Object Reference" :default "/Game/ATG_Testing/ParkourMovement/IA_Sprint.IA_Sprint"))
  (:`Triggered`
    (`ParkourMovementComponent.Sprint` (`self.ParkourMovementSystem`))))

(event `EnhancedInput|/Game/ATG_Testing/GameplayAbilitySystem/IA_Punch`
  (params (ActionValue :type Boolean) (ElapsedSeconds :type "Float (double-precision)") (TriggeredSeconds :type "Float (double-precision)") (InputAction :type "InputAction Object Reference" :default "/Game/ATG_Testing/GameplayAbilitySystem/IA_Punch.IA_Punch"))
  (:`Triggered`
    (`AbilitySystemComponent.TryActivateAbilityByClass` (`self.AbilitySystemComponent`) "/Game/ATG_Testing/GameplayAbilitySystem/GA_Punch.GA_Punch_C" true)))

(event `Handle Punch`
  (bind _returnvalue (`self.GetInstigator`))
  (bind _outactors (`KismetSystemLibrary.SphereOverlapActors` (`SceneComponent.GetSocketLocation` (`self.Mesh`) "hand_r") 50.0 (`|MakeArray` "ObjectTypeQuery3" :!type "EObjectTypeQuery Enum") "BP_TPC_Testing_C" (`|MakeArray` self :!type "Actor Object Reference")))
  (if (`KismetArrayLibrary.Array_IsValidIndex` _outactors)
    (bind _output (`|GetArrayItem` _outactors))
    (`AbilitySystemBlueprintLibrary.SendGameplayEventToActor` _returnvalue (struct :`TagName` "Reub.Weapon.Hit") (make `GameplayEventData` (struct) _returnvalue _output null null (struct) (struct) (struct) 0.0 (`AbilitySystemBlueprintLibrary.AbilityTargetDataFromActor` _output)))))

(fn `UserConstructionScript`
  (`SkinnedMeshComponent.SetLeaderPoseComponent` (`self.HelmetMesh`) (`self.Mesh`) false false)
  (`SkinnedMeshComponent.SetLeaderPoseComponent` (`self.VestMesh`) (`self.Mesh`) false false))